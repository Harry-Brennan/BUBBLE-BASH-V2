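; BP_Bounce_Pad is a bounce pad hazard that launches overlapping actors with a primitive root component along its BounceDirection.
; On overlap it restores the X and Y velocity reported by the actor's GetLastVelocityCheckMessage, dropping vertical motion.
; It then adds a mass-independent impulse scaled by ForceAmount.
; Actors implementing BPI_Player also have their BPC_Dash up and down dashes reset.
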(event `self.Bounce Pad Activation Collision.OnComponentBeginOverlap`
  (params (OverlappedComponent :type "PrimitiveComponent Object Reference") (OtherActor :type "Actor Object Reference") (OtherComp :type "PrimitiveComponent Object Reference") (OtherBodyIndex :type Integer) (bFromSweep :type Boolean) (SweepResult :type "HitResult Structure (by ref)"))
  (bind _returnvalue (`self.GetComponentByClass` OtherActor "/Game/Player/In-Round/BPC_Dash.BPC_Dash_C"))
  (bind _asprimitive_component (cast `PrimitiveComponent` (`Actor.RootComponent` OtherActor)))
  (bind _velocity (message `/Game/Player/In-Round/BPI_Player.Get Last Velocity Check` OtherActor))
  (`PrimitiveComponent.SetAllPhysicsLinearVelocity` _asprimitive_component (`KismetMathLibrary.MakeVector` (.x _velocity) (.y _velocity)) false)
  (`PrimitiveComponent.AddImpulse` _asprimitive_component (* (`SceneComponent.GetForwardVector` (`self.Bounce Direction`)) (`self.Force Amount`)) "None" true)
  (if (`KismetSystemLibrary.DoesImplementInterface` OtherActor "/Game/Player/In-Round/BPI_Player.BPI_Player_C")
    (`/Game/Player/In-Round/BPC_Dash.Reset Dash Down Done` _returnvalue)
    (`/Game/Player/In-Round/BPC_Dash.Reset Dash Up Done` _returnvalue)))

(fn `UserConstructionScript`)