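; Toggleable hazard volume that pushes overlapping actors along its ForceDirection, with debug prints.
; Overlap starts a looping timer that applies mass-independent force to each actor's root primitive.
; Optional clamped falloff scales force by centre distance over capsule radius, horizontal or 3D.
; The timer clears when the volume empties or ticks while inactive; only a new overlap restarts it, not reactivation.
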(event `Activate Push Volume`
  (set `self.Active` true))

(event `Deactivate Push Volume`
  (set `self.Active` false))

(event `self.Push Collision.OnComponentBeginOverlap`
  (params (OverlappedComponent :type "PrimitiveComponent Object Reference") (OtherActor :type "Actor Object Reference") (OtherComp :type "PrimitiveComponent Object Reference") (OtherBodyIndex :type Integer) (bFromSweep :type Boolean) (SweepResult :type "HitResult Structure (by ref)"))
  (`KismetSystemLibrary.PrintString` (`KismetSystemLibrary.GetDisplayName` OtherComp))
  (`KismetArrayLibrary.Array_Add` (`self.Overlapping Actors`) OtherActor)
  (if (not (`KismetSystemLibrary.K2_IsValidTimerHandle` (`self.Push Loop Timer`)))
    (bind _returnvalue (`KismetSystemLibrary.K2_SetTimerDelegate` (delegate `Push Loop`) 0.05 true))
    (set `self.Push Loop Timer` _returnvalue)))

(event `Push Loop`
  (bind (_returnvalue_x _returnvalue_y) (`KismetMathLibrary.BreakVector` (`self.K2_GetActorLocation`)))
  (bind (_returnvalue_x_2 _returnvalue_y_2 _returnvalue_z) (`KismetMathLibrary.BreakVector` (`self.K2_GetActorLocation`)))
  (if (`self.Active`)
    (for _array_element (`self.Overlapping Actors`)
      (bind (_returnvalue_x_3 _returnvalue_y_3 _returnvalue_z_2) (`KismetMathLibrary.BreakVector` (`self.K2_GetActorLocation` _array_element)))
      (bind (_returnvalue_x_4 _returnvalue_y_4) (`KismetMathLibrary.BreakVector` (`self.K2_GetActorLocation` _array_element)))
      (bind _returnvalue (`KismetMathLibrary.FClamp` (+ (- 1.0 (/ (`KismetMathLibrary.SelectFloat` (`KismetMathLibrary.SelectFloat` (`KismetMathLibrary.Vector_Distance` (`self.K2_GetActorLocation` _array_element) (`self.K2_GetActorLocation`)) (- _returnvalue_z_2 _returnvalue_z) (`self.Force Relative to Centre Distance XY`)) (`KismetMathLibrary.Vector_Distance` (`KismetMathLibrary.MakeVector` _returnvalue_x _returnvalue_y) (`KismetMathLibrary.MakeVector` _returnvalue_x_4 _returnvalue_y_4)) (`self.Force Relative to Centre Distance Z`)) (`CapsuleComponent.GetScaledCapsuleSize` (`self.Push Collision`)))) 0.25) 0.1))
      (`KismetSystemLibrary.PrintString` (`KismetStringLibrary.Conv_DoubleToString` _returnvalue))
      (bind _asprimitive_component (cast `PrimitiveComponent` (`Actor.RootComponent` _array_element)))
      (`PrimitiveComponent.AddForce` _asprimitive_component (* (`SceneComponent.GetForwardVector` (`self.Force Direction`)) (`self.Force Amount`) (`KismetMathLibrary.SelectFloat` _returnvalue 1.0 (`self.Force Relative to Centre Distance XY`))) "None" true))
    (else
      (`KismetSystemLibrary.K2_ClearAndInvalidateTimerHandle` (`self.Push Loop Timer`)))))

(event `self.Push Collision.OnComponentEndOverlap`
  (params (OverlappedComponent :type "PrimitiveComponent Object Reference") (OtherActor :type "Actor Object Reference") (OtherComp :type "PrimitiveComponent Object Reference") (OtherBodyIndex :type Integer))
  (`KismetArrayLibrary.Array_RemoveItem` (`self.Overlapping Actors`) OtherActor)
  (if (`KismetArrayLibrary.Array_IsEmpty` (`self.Overlapping Actors`))
    (`KismetSystemLibrary.K2_ClearAndInvalidateTimerHandle` (`self.Push Loop Timer`))))

(fn `UserConstructionScript`)