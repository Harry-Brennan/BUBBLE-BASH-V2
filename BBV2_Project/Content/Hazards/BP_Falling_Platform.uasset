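; BP_Falling_Platform is a hazard platform that drops under physics shortly after its activation collision is overlapped.
; An overlap starts a one-shot delay timer, unless one is already pending or the mesh is simulating, which then enables physics on the mass-overridden static mesh.
; A reset event stops simulation, clears the timer and teleports the actor back to the transform cached at BeginPlay.
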(event `self.ReceiveBeginPlay`
  (set `self.Starting Transform` (`self.GetTransform`))
  (`PrimitiveComponent.SetMassOverrideInKg` (`self.Falling Platform SM`) "None" (`self.Platform Mass`) true))

(event `Reset Falling Platform`
  (`PrimitiveComponent.SetSimulatePhysics` (`self.Falling Platform SM`) false)
  (`KismetSystemLibrary.K2_ClearAndInvalidateTimerHandle` (`self.Fall Timer`))
  (`self.K2_SetActorTransform` (`self.Starting Transform`) false true))

(event `Falling Platform Activate`
  (`PrimitiveComponent.SetSimulatePhysics` (`self.Falling Platform SM`) true))

(event `self.Falling Platform Activation Collision.OnComponentBeginOverlap`
  (params (OverlappedComponent :type "PrimitiveComponent Object Reference") (OtherActor :type "Actor Object Reference") (OtherComp :type "PrimitiveComponent Object Reference") (OtherBodyIndex :type Integer) (bFromSweep :type Boolean) (SweepResult :type "HitResult Structure (by ref)"))
  (if (not (or (`KismetSystemLibrary.K2_IsValidTimerHandle` (`self.Fall Timer`)) (`SceneComponent.IsSimulatingPhysics` (`self.Falling Platform SM`) "None")))
    (bind _returnvalue (`KismetSystemLibrary.K2_SetTimerDelegate` (delegate `Falling Platform Activate`) (`self.Fall Activate Delay Time`)))
    (set `self.Fall Timer` _returnvalue)))

(fn `UserConstructionScript`)