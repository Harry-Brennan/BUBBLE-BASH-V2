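; Player drop-shadow actor that marks the surface below its owner while airborne.
; Each tick it line-traces along the negative up vector of the owner's orientation indicator, moves to the hit, and smoothly grows the flattened shadow mesh with distance.
; It collapses the mesh to zero scale when the owner reports being grounded; activate and deactivate events toggle ticking.
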(event `self.ReceiveBeginPlay`
  (bind _static_mesh_component (message `/Game/Player/BPI_Player.Get Standard Orientation Indicator` (`self.GetOwner`)))
  (set `self.Owner's Standard Orientation Indicator` _static_mesh_component))

(event `Activate Shadow`
  (`self.SetActorTickEnabled` true))

(event `Deactivate Shadow`
  (`self.SetActorTickEnabled` false)
  (`SceneComponent.SetWorldScale3D` (`self.Shadow SM`) (0.0 0.0 0.0)))

(event `self.ReceiveTick`
  (params (DeltaSeconds :type "Float (single-precision)"))
  (bind _returnvalue (`GameplayStatics.GetWorldDeltaSeconds`))
  (bind (_returnvalue_x _returnvalue_y) (`KismetMathLibrary.BreakVector` (`SceneComponent.K2_GetComponentScale` (`self.Shadow SM`))))
  (bind _returnvalue_2 (`self.K2_GetActorLocation` (`self.GetOwner`)))
  (`/Engine/EditorBlueprintResources/StandardMacros.IsValid` (`self.GetOwner`)
    (:`Is Valid`
      (bind _on_ground (message `/Game/Player/BPI_Player.Get On Ground` (`self.GetOwner`)))
      (if _on_ground
        (`SceneComponent.SetWorldScale3D` (`self.Shadow SM`) (0.0 0.0 0.0))
        (else
          (bind _outhit (`KismetSystemLibrary.LineTraceSingleForObjects` _returnvalue_2 (+ _returnvalue_2 (* (`SceneComponent.GetUpVector` (`self.Owner's Standard Orientation Indicator`)) -9999.0)) (`|MakeArray` "ObjectTypeQuery1" "ObjectTypeQuery2" "ObjectTypeQuery4" :!type "EObjectTypeQuery Enum")))
          (bind (_bblockinghit _binitialoverlap _time _distance _location) (`GameplayStatics.BreakHitResult` _outhit))
          (`self.K2_SetActorLocation` _location)
          (bind _returnvalue_3 (`KismetMathLibrary.MapRangeClamped` _distance 500.0 2500.0 0.0 4.0))
          (`SceneComponent.SetWorldScale3D` (`self.Shadow SM`) (`KismetMathLibrary.MakeVector` (`KismetMathLibrary.FInterpTo` _returnvalue_x _returnvalue_3 _returnvalue 25.0) (`KismetMathLibrary.FInterpTo` _returnvalue_y _returnvalue_3 _returnvalue 25.0) 0.01)))))))

(fn `UserConstructionScript`)