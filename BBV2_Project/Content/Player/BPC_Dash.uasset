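; Player dash component that gives its owning Character horizontal, upward and downward dashes from Enhanced Input actions.
; Dash applies a velocity-change impulse to the capsule, scaled by the bubble amount, zeroing existing velocity first above a threshold, then drives the buildup toward zero.
; Horizontal dashes follow last movement input, while vertical ones follow the orientation indicator's up axis.
; Each vertical dash works once until externally reset, and downward requires being airborne.
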(event `self.ReceiveBeginPlay`
  (bind _ascharacter (cast `Character` (`self.GetOwner`)))
  (set `self.Owner as Character` _ascharacter))

(event `EnhancedInput|/Game/Player/Input/Actions/In_Round/Dashing/IA_Horizontal_Dash`
  (params (ActionValue :type Boolean) (ElapsedSeconds :type "Float (double-precision)") (TriggeredSeconds :type "Float (double-precision)") (InputAction :type "InputAction Object Reference" :default "/Game/Player/Input/Actions/In_Round/Dashing/IA_Horizontal_Dash.IA_Horizontal_Dash"))
  (:`Triggered`
    (bind _last_movement_input_vector (message `/Game/Player/BPI_Player.Get Last Movement Input Vector` (`self.Owner as Character`)))
    (`self.Dash` _last_movement_input_vector true)))

(event `EnhancedInput|/Game/Player/Input/Actions/In_Round/Dashing/IA_Vertical_Dash_Down`
  (params (ActionValue :type Boolean) (ElapsedSeconds :type "Float (double-precision)") (TriggeredSeconds :type "Float (double-precision)") (InputAction :type "InputAction Object Reference" :default "/Game/Player/Input/Actions/In_Round/Dashing/IA_Vertical_Dash_Down.IA_Vertical_Dash_Down"))
  (:`Triggered`
    (bind _on_ground (message `/Game/Player/BPI_Player.Get On Ground` (`self.Owner as Character`)))
    (if (and (not _on_ground) (not (`self.Dash Down Done`)))
      (bind _static_mesh_component (message `/Game/Player/BPI_Player.Get Standard Orientation Indicator` (`self.Owner as Character`)))
      (`self.Dash` (* (`SceneComponent.GetUpVector` _static_mesh_component) -1.0))
      (set `self.Dash Down Done` true))))

(event `EnhancedInput|/Game/Player/Input/Actions/In_Round/Dashing/IA_Vertical_Dash_Up`
  (params (ActionValue :type Boolean) (ElapsedSeconds :type "Float (double-precision)") (TriggeredSeconds :type "Float (double-precision)") (InputAction :type "InputAction Object Reference" :default "/Game/Player/Input/Actions/In_Round/Dashing/IA_Vertical_Dash_Up.IA_Vertical_Dash_Up"))
  (:`Triggered`
    (bind _static_mesh_component (message `/Game/Player/BPI_Player.Get Standard Orientation Indicator` (`self.Owner as Character`)))
    (if (not (`self.Dash Up Done`))
      (`self.Dash` (`SceneComponent.GetUpVector` _static_mesh_component))
      (set `self.Dash Up Done` true))))

(fn `Dash`
  (params (`Dash Direction` :type "Vector Structure") (`Dash Horizontal?` :type Boolean))
  (bind _capsulecomponent (`Character.CapsuleComponent` (`self.Owner as Character`)))
  (bind _current_bubble_amount (message `/Game/Player/BPI_Player.Get Current Bubble Amount` (`self.Owner as Character`)))
  (if (> _current_bubble_amount (`KismetMathLibrary.SelectFloat` (`self.Stopping Buildup Requirement Horizontal`) (`self.Stopping Buildup Requirement Vertical`) (`local.Dash Horizontal?`)))
    (`PrimitiveComponent.SetPhysicsLinearVelocity` _capsulecomponent (0.0 0.0 0.0) false "None"))
  (`PrimitiveComponent.AddImpulse` _capsulecomponent (* (`KismetMathLibrary.GetForwardVector` (`KismetMathLibrary.MakeRotFromX` `Dash Direction`)) (`KismetMathLibrary.SelectFloat` (`KismetMathLibrary.Lerp` (`self.Min Dash Force`) (`self.Max Dash Force`) _current_bubble_amount) (`KismetMathLibrary.Lerp` (`self.Min Vertical Dash Force`) (`self.Max Vertical Dash Force`) _current_bubble_amount) (`local.Dash Horizontal?`))) "None" true)
  (message `/Game/Player/BPI_Player.Update Alternative Target Buildup` (`self.Owner as Character`) 0.0 1.0 10.0))

(fn `Reset Dash Down Done`
  (set `self.Dash Down Done` false))

(fn `Reset Dash Up Done`
  (set `self.Dash Up Done` false))