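; Handler that applies physics knockback to two players when they collide above a minimum combined velocity.
; PlayerKnockbackActivate keeps parallel arrays of player pairs and timestamps to block repeat hits from the same pair, in either order, within a cooldown.
; Valid hits impulse both root components using velocities mirrored by the hit normal, negated for the hitter and scaled per role.
; Persistent debug line traces visualize each impulse.
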(fn `Player Knockback Activate`
  (params (`Hit Player` :type "Actor Object Reference") (`Player who hit` :type "Actor Object Reference") (`Velocity of player who hit` :type "Vector Structure") (`Velocity of player who was hit` :type "Vector Structure") (`Hit Normal` :type "Vector Structure"))
  (bind _struct_player_to_player_knockback_info (make `/Game/Player/Player_to_Player_Knockback/Struct_Player_to_Player_Knockback_Info` `Player who hit` `Hit Player`))
  (bind _struct_player_to_player_knockback_info_2 (make `/Game/Player/Player_to_Player_Knockback/Struct_Player_to_Player_Knockback_Info` `Hit Player` `Player who hit`))
  (bind _returnvalue (`KismetArrayLibrary.Array_Find` (`self.Stored Player Knockback Info`) _struct_player_to_player_knockback_info))
  (bind _returnvalue_2 (`KismetArrayLibrary.Array_Find` (`self.Stored Player Knockback Info`) _struct_player_to_player_knockback_info_2))
  (bind _returnvalue_3 (`self.K2_GetActorLocation` (`local.Hit Player`)))
  (bind _returnvalue_4 (`self.K2_GetActorLocation` (`local.Player who hit`)))
  (bind _returnvalue_5 (`KismetMathLibrary.MirrorVectorByNormal` (* (`local.Velocity of player who hit`) (`self.Player Who got Hit Knockback Multiplier`)) (`local.Hit Normal`)))
  (bind _returnvalue_6 (* (`KismetMathLibrary.NegateVector` (`KismetMathLibrary.MirrorVectorByNormal` (+ (`local.Velocity of player who hit`) (`local.Velocity of player who was hit`)) (`local.Hit Normal`))) (`self.Player Who Hit Knockback Multiplier`)))
  (if (>= (`KismetMathLibrary.VSize` (+ (`local.Velocity of player who hit`) (`local.Velocity of player who was hit`))) (`self.Min Combined Velocity for Activation`))
    (if (`KismetArrayLibrary.Array_Contains` (`self.Stored Player Knockback Info`) _struct_player_to_player_knockback_info_2)
      (if (>= (- (`KismetSystemLibrary.GetGameTimeInSeconds`) (`|GetArrayItem` (`self.Player Knockback Times`) _returnvalue_2)) (`self.Min Time Since Last Duplicate Knockback Instance`))
        (`KismetArrayLibrary.Array_Remove` (`self.Player Knockback Times`) _returnvalue_2)
        (`KismetArrayLibrary.Array_RemoveItem` (`self.Stored Player Knockback Info`) (`|GetArrayItem` (`self.Stored Player Knockback Info`) _returnvalue_2))
        (`KismetArrayLibrary.Array_Add` (`self.Stored Player Knockback Info`) (make `/Game/Player/Player_to_Player_Knockback/Struct_Player_to_Player_Knockback_Info` (`local.Hit Player`) (`local.Player who hit`)) :!label _label)
        (`KismetArrayLibrary.Array_Add` (`self.Player Knockback Times`) (`KismetSystemLibrary.GetGameTimeInSeconds`))
        (bind _asprimitive_component (cast `PrimitiveComponent` (`Actor.RootComponent` (`local.Hit Player`))))
        (`PrimitiveComponent.AddImpulse` _asprimitive_component _returnvalue_5 "None" false)
        (`KismetSystemLibrary.LineTraceSingle` :`Start` _returnvalue_3 :`End` (+ _returnvalue_3 _returnvalue_5) :`TraceChannel` "TraceTypeQuery1" :`DrawDebugType` "Persistent")
        (bind _asprimitive_component_2 (cast `PrimitiveComponent` (`Actor.RootComponent` (`local.Player who hit`))))
        (`PrimitiveComponent.AddImpulse` _asprimitive_component_2 _returnvalue_6 "None" false)
        (`KismetSystemLibrary.LineTraceSingle` :`Start` _returnvalue_4 :`End` (+ _returnvalue_4 _returnvalue_6) :`TraceChannel` "TraceTypeQuery1" :`DrawDebugType` "Persistent"))
      (elif (`KismetArrayLibrary.Array_Contains` (`self.Stored Player Knockback Info`) _struct_player_to_player_knockback_info)
        (if (>= (- (`KismetSystemLibrary.GetGameTimeInSeconds`) (`|GetArrayItem` (`self.Player Knockback Times`) _returnvalue)) (`self.Min Time Since Last Duplicate Knockback Instance`))
          (`KismetArrayLibrary.Array_Remove` (`self.Player Knockback Times`) _returnvalue)
          (`KismetArrayLibrary.Array_RemoveItem` (`self.Stored Player Knockback Info`) (`|GetArrayItem` (`self.Stored Player Knockback Info`) _returnvalue))
          (goto _label))
        (else
          (goto _label))))))

(fn `UserConstructionScript`)