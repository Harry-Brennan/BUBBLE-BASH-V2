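; Player camera actor that follows a target actor (initially its owner) in one of three modes: controllable third person, stationary, or spline based.
; Third person rotates the boom from owner axis input, with follow speeds and arm length scaled by distance and velocity, plus a timed arm-length override.
; Stationary snaps to a setup actor while the player lives; spline mode maps target progress onto a location spline with clamped look-at.
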(event `self.ReceiveBeginPlay`
  (bind _output_get (set `self.Target Actor` (`self.GetOwner`)))
  (set `self.Owning Player` _output_get)
  (bind _returnvalue (`GameplayStatics.GetActorOfClass` "/Game/Player/Camera/BP_Camera_Location_Spline.BP_Camera_Location_Spline_C"))
  (set `self.Linked Location Spline` _returnvalue)
  (bind _returnvalue_2 (`GameplayStatics.GetActorOfClass` "/Game/Player/Camera/BP_Camera_Player_Distance_Spline.BP_Camera_Player_Distance_Spline_C"))
  (set `self.Linked Distance Spline` _returnvalue_2)
  (bind _returnvalue_3 (`GameplayStatics.GetActorOfClass` "/Game/Player/Camera/BP_Camera_Stationary_Setup.BP_Camera_Stationary_Setup_C"))
  (set `self.Linked Camera Stationary Setup` _returnvalue_3))

(event `Update Target Actor`
  (params (`New Target` :type "Actor Object Reference"))
  (set `self.Target Actor` `New Target`)
  (`self.SetActorTickEnabled` true))

(event `Update Camera Mode`
  (params (`New Mode` :type "/Game/Player/Camera/Enum_Camera_Modes Enum" :default "NewEnumerator0"))
  (set `self.Current Camera Mode` `New Mode`)
  (`self.SetActorTickEnabled` true))

(event `End Alternative Target Arm Length Activity`
  (set `self.Alternative Target Arm Length Active` false))

(event `Update Alternative Target Arm Length`
  (params (`New Percentage` :type "Float (double-precision)") (`Time until Back to Normal` :type "Float (double-precision)"))
  (`KismetSystemLibrary.K2_ClearAndInvalidateTimerHandle` (`self.End Alternative Target Arm Length Activity Timer`))
  (set `self.Alternative Target Arm Length Active` true)
  (set `self.Alternative Target Arm Length` (`KismetMathLibrary.Lerp` (/ (`self.Min Arm Length`) 2.0) (`self.Max Arm Length`) `New Percentage`))
  (bind _returnvalue (`KismetSystemLibrary.K2_SetTimerDelegate` (delegate `End Alternative Target Arm Length Activity`) `Time until Back to Normal`))
  (set `self.End Alternative Target Arm Length Activity Timer` _returnvalue))

(event `self.ReceiveTick`
  (params (DeltaSeconds :type "Float (single-precision)"))
  (bind (_returnvalue_x _returnvalue_y) (`KismetMathLibrary.BreakVector` (`self.K2_GetActorLocation`)))
  (bind _returnvalue (`GameplayStatics.GetWorldDeltaSeconds`))
  (bind (_returnvalue_roll _returnvalue_pitch _returnvalue_yaw) (`KismetMathLibrary.BreakRotator` (`self.K2_GetActorRotation`)))
  (bind (_returnvalue_location _returnvalue_rotation) (`KismetMathLibrary.BreakTransform` (`self.GetTransform` (`self.Linked Camera Stationary Setup`))))
  (bind (_returnvalue_x_2 _returnvalue_y_2 _returnvalue_z) (`KismetMathLibrary.BreakVector` (`self.GetVelocity` (`self.Target Actor`))))
  (bind (_returnvalue_x_3 _returnvalue_y_3) (`KismetMathLibrary.BreakVector` (`self.K2_GetActorLocation` (`self.Target Actor`))))
  (bind (_returnvalue_x_4 _returnvalue_y_4 _returnvalue_z_2) (`KismetMathLibrary.BreakVector` (`self.GetVelocity` (`self.Target Actor`))))
  (bind (_returnvalue_x_5 _returnvalue_y_5) (`KismetMathLibrary.BreakVector` (`self.K2_GetActorLocation` (`self.Target Actor`))))
  (bind (_returnvalue_x_6 _returnvalue_y_6 _returnvalue_z_3) (`KismetMathLibrary.BreakVector` (`self.GetVelocity` (`self.Target Actor`))))
  (bind (_returnvalue_roll_2 _returnvalue_pitch_2 _returnvalue_yaw_2) (`KismetMathLibrary.BreakRotator` (`KismetMathLibrary.FindLookAtRotation` (`self.K2_GetActorLocation`) (`self.K2_GetActorLocation` (`self.Target Actor`)))))
  (bind (_returnvalue_roll_3 _returnvalue_pitch_3 _returnvalue_yaw_3) (`KismetMathLibrary.BreakRotator` (`KismetMathLibrary.FindLookAtRotation` (`SplineComponent.GetLocationAtDistanceAlongSpline` (`/Game/Player/Camera/BP_Camera_Location_Spline.Camera Location Spline` (`self.Linked Location Spline`)) 0.0 "World") (`SplineComponent.GetLocationAtDistanceAlongSpline` (`/Game/Player/Camera/BP_Camera_Player_Distance_Spline.Distance Calculating Spline` (`self.Linked Distance Spline`)) 0.0 "World"))))
  (bind (_returnvalue_x_7 _returnvalue_y_7) (`KismetMathLibrary.BreakVector` (`KismetMathLibrary.VInterpTo` (`self.K2_GetActorLocation`) (`self.K2_GetActorLocation` (`self.Target Actor`)) (`GameplayStatics.GetWorldDeltaSeconds`) (`KismetMathLibrary.MapRangeClamped` (`KismetMathLibrary.Vector_Distance` (`KismetMathLibrary.MakeVector` _returnvalue_x _returnvalue_y) (`KismetMathLibrary.MakeVector` _returnvalue_x_3 _returnvalue_y_3)) 0.0 (`self.Max XY Velocity Range`) (`self.Min Camera XY Move Speed`) (`self.Max Camera XY Move Speed`)))))
  (bind (_returnvalue_x_8 _returnvalue_y_8 _returnvalue_z_4) (`KismetMathLibrary.BreakVector` (`KismetMathLibrary.VInterpTo` (`self.K2_GetActorLocation`) (`self.K2_GetActorLocation` (`self.Target Actor`)) (`GameplayStatics.GetWorldDeltaSeconds`) (`KismetMathLibrary.SelectFloat` (`KismetMathLibrary.MapRangeClamped` (`KismetMathLibrary.VSize` (`KismetMathLibrary.MakeVector` _returnvalue_z_2)) 0.0 (`self.Max Z Velocity Range`) (`self.Min Camera Z Move Speed`) (`self.Max Camera Z Move Speed`)) 15.0 (== (`self.Owning Player`) (`self.Target Actor`))))))
  (`self.Target Actor`
    (:`then`
      (switch `/Game/Player/Camera/Enum_Camera_Modes` (`self.Current Camera Mode`)
        (:`NewEnumerator0`
          (bind (_y _z) (message `/Game/Player/BPI_Player.Get Camera Axis Values` (`self.Owning Player`) :!label _label))
          (`SceneComponent.K2_SetRelativeRotation` (`self.Camera Boom`) (`CustomFunctions.RInterpToConstant` (`SceneComponent.RelativeRotation` (`self.Camera Boom`)) (`KismetMathLibrary.MakeRotator` 0.0 _y _z) (`GameplayStatics.GetWorldDeltaSeconds`) (`self.Rotation Speed`) true) false false)
          (set `SpringArmComponent.TargetArmLength` (`KismetMathLibrary.FInterpTo` (`SpringArmComponent.TargetArmLength` (`self.Camera Boom`)) (`KismetMathLibrary.SelectFloat` (`self.Alternative Target Arm Length`) (`KismetMathLibrary.MapRangeClamped` (`KismetMathLibrary.VSize` (`KismetMathLibrary.MakeVector` _returnvalue_x_6 _returnvalue_y_6 (/ _returnvalue_z_3 (`self.Arm Length Z Velocity Division Factor`)))) 0.0 (`self.Max Velocity Arm Equivalent`) (`self.Min Arm Length`) (`self.Max Arm Length`)) (`self.Alternative Target Arm Length Active`)) (`GameplayStatics.GetWorldDeltaSeconds`) (`self.Arm Length Interp Speed`)) (`self.Camera Boom`))
          (`self.K2_SetActorLocation` (`KismetMathLibrary.MakeVector` _returnvalue_x_7 _returnvalue_y_7 _returnvalue_z_4)))
        (:`NewEnumerator1`
          (if (`/Game/Player/Health_And_Death/BPC_Player_Health.Player Alive?` (`self.GetComponentByClass` (`self.Owning Player`) "/Game/Player/Health_And_Death/BPC_Player_Health.BPC_Player_Health_C"))
            (`self.K2_SetActorLocationAndRotation` _returnvalue_location _returnvalue_rotation)
            (set `SpringArmComponent.TargetArmLength` (`SpringArmComponent.TargetArmLength` (`/Game/Player/Camera/BP_Camera_Stationary_Setup.SpringArm` (`self.Linked Camera Stationary Setup`))) (`self.Camera Boom`))
            (`KismetSystemLibrary.Delay` 0.2)
            (`self.SetActorTickEnabled` false)
            (else
              (goto _label))))
        (:`NewEnumerator2`
          (`/Engine/EditorBlueprintResources/StandardMacros.IsValid` (`self.Linked Location Spline`)
            (:`Is Valid`
              (`/Engine/EditorBlueprintResources/StandardMacros.IsValid` (`self.Linked Distance Spline`)
                (:`Is Valid`
                  (set `self.Current Spline Distance` (`SplineComponent.GetDistanceAlongSplineAtLocation` (`/Game/Player/Camera/BP_Camera_Player_Distance_Spline.Distance Calculating Spline` (`self.Linked Distance Spline`)) (`KismetMathLibrary.MakeVector` _returnvalue_x_5 _returnvalue_y_5) "World"))
                  (`self.K2_SetActorLocationAndRotation` (`KismetMathLibrary.VInterpTo` (`self.K2_GetActorLocation`) (`SplineComponent.GetLocationAtDistanceAlongSpline` (`/Game/Player/Camera/BP_Camera_Location_Spline.Camera Location Spline` (`self.Linked Location Spline`)) (`self.Current Spline Distance`) "World") (`GameplayStatics.GetWorldDeltaSeconds`) 5.0) (`KismetMathLibrary.MakeRotator` 0.0 (`KismetMathLibrary.FClamp` (`KismetMathLibrary.FInterpTo` _returnvalue_pitch _returnvalue_pitch_2 _returnvalue 3.0) (- _returnvalue_pitch_3 45.0) (+ _returnvalue_pitch_3 60.0)) (`KismetMathLibrary.FClamp` (`KismetMathLibrary.FInterpTo` _returnvalue_yaw _returnvalue_yaw_2 _returnvalue 5.0) (- _returnvalue_yaw_3 45.0) (+ _returnvalue_yaw_3 45.0))))
                  (set `SpringArmComponent.TargetArmLength` (`KismetMathLibrary.FInterpTo` (`SpringArmComponent.TargetArmLength` (`self.Camera Boom`)) (`KismetMathLibrary.SelectFloat` (`self.Alternative Target Arm Length`) (`KismetMathLibrary.MapRangeClamped` (`KismetMathLibrary.VSize` (`KismetMathLibrary.MakeVector` _returnvalue_x_2 _returnvalue_y_2 (/ _returnvalue_z (`self.Arm Length Z Velocity Division Factor`)))) 0.0 (`self.Max Velocity Arm Equivalent`) (`self.Min Arm Length`) (`self.Max Arm Length`)) (`self.Alternative Target Arm Length Active`)) (`GameplayStatics.GetWorldDeltaSeconds`) (`self.Arm Length Interp Speed`)) (`self.Camera Boom`)))
                (:`Is Not Valid`
                  (goto _label))))
            (:`Is Not Valid`
              (goto _label))))))
    (:`else`)))

(fn `UserConstructionScript`)