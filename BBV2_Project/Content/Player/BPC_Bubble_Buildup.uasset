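; Player component that grows and shrinks its owning bubble actor according to how fast it moves.
; Each tick, speed, scaled against separate ground and air maximums, nudges a clamped 0–1 buildup up or down with its own interp speeds.
; Buildup drives the actor's scale and, very slightly, its root capsule size.
; A timed override can instead pull buildup toward a given target at a given speed until its timer expires.
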(event `self.ReceiveBeginPlay`
  (bind _ascapsule_collision (cast `CapsuleComponent` (`Actor.RootComponent` (`self.GetOwner`))))
  (set `self.Owners Capsule Collision` _ascapsule_collision))

(event `self.ReceiveTick`
  (params (DeltaSeconds :type "Float (single-precision)"))
  (bind _current_bubble_buildup (`self.Current Bubble Buildup`))
  (bind _max_velocity_on_ground (`self.Max Velocity On Ground`))
  (bind _on_ground (message `/Game/Player/BPI_Player.Get On Ground` (`self.GetOwner`)))
  (bind _returnvalue (`KismetMathLibrary.MapRangeClamped` (`KismetMathLibrary.VSize` (`Actor.GetVelocity` (`self.GetOwner`))) 0.0 (`KismetMathLibrary.SelectFloat` _max_velocity_on_ground (* _max_velocity_on_ground (`self.In Air Max Velocity Multiplier`)) _on_ground) (`self.Negative Buildup Interval`) (`self.Positive Buildup Interval`)))
  (`self.Update Bubble Buildup Amount` (`KismetMathLibrary.FInterpTo` _current_bubble_buildup (`KismetMathLibrary.SelectFloat` (`self.Alternative Target Buildup`) (+ _current_bubble_buildup _returnvalue) (`self.Buildup Alternative Active`)) (`GameplayStatics.GetWorldDeltaSeconds`) (`KismetMathLibrary.SelectFloat` (`self.Alterative Target Buildup Speed`) (`KismetMathLibrary.SelectFloat` (`self.Negative Buildup Speed`) (`self.Positive Buildup Speed`) (< _returnvalue 0.0)) (`self.Buildup Alternative Active`)))))

(fn `Disable Alternative Buildup`
  (set `self.Buildup Alternative Active` false))

(fn `Update Alternative Target Buildup`
  (params (`New Alternative Buildup Amount` :type "Float (double-precision)") (`How Long Should Alternative Be Active` :type "Float (double-precision)") (`Target Buildup Speed` :type "Float (double-precision)"))
  (`KismetSystemLibrary.K2_ClearAndInvalidateTimerHandle` (`self.Disable Alternative Buildup Timer`))
  (set `self.Alternative Target Buildup` `New Alternative Buildup Amount`)
  (set `self.Alterative Target Buildup Speed` `Target Buildup Speed`)
  (set `self.Buildup Alternative Active` true)
  (bind _returnvalue (`KismetSystemLibrary.K2_SetTimer` null "Disable Alternative Buildup" `How Long Should Alternative Be Active`))
  (set `self.Disable Alternative Buildup Timer` _returnvalue))

(fn `Update Bubble Buildup Amount`
  (params (`New Buildup Amount` :type "Float (double-precision)"))
  (set `self.Current Bubble Buildup` (`KismetMathLibrary.FClamp` `New Buildup Amount`))
  (`self.Update Bubble Scale`))

(fn `Update Bubble Scale`
  (bind _current_bubble_buildup (`self.Current Bubble Buildup`))
  (bind _returnvalue (`KismetMathLibrary.Lerp` 160.0 160.5 _current_bubble_buildup))
  (`Actor.SetActorScale3D` (`self.GetOwner`) (`KismetMathLibrary.VLerp` (`self.Min Bubble Scale`) (`self.Max Bubble Scale`) _current_bubble_buildup))
  (`CapsuleComponent.SetCapsuleSize` (`self.Owners Capsule Collision`) _returnvalue _returnvalue false))