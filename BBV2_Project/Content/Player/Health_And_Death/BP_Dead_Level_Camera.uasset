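; Level camera for player death that rotates a boom-mounted camera, either freely or between preset views.
; Activate and Deactivate toggle Tick, which interpolates the boom toward the player's camera axis values when rotation is allowed or no presets exist.
; Otherwise it eases toward the current preset, which next/previous events cycle with wraparound.
; Helpers select the preset nearest the current rotation, or test each to find the camera position nearest the dead body.
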(event `self.ReceiveBeginPlay`
  (set `self.Owning Player` (`GameplayStatics.GetPlayerCharacter` 0)))

(event `Activate Dead Level Cam`
  (`self.SetActorTickEnabled` true))

(event `Deactivate Dead Level Cam`
  (`self.SetActorTickEnabled` false))

(event `self.ReceiveTick`
  (params (DeltaSeconds :type "Float (single-precision)"))
  (bind (_relativerotation_roll _relativerotation_pitch _relativerotation_yaw) (`KismetMathLibrary.BreakRotator` (`SceneComponent.RelativeRotation` (`self.Camera Boom`))))
  (bind (_returnvalue_roll _returnvalue_pitch _returnvalue_yaw) (`KismetMathLibrary.BreakRotator` (`KismetMathLibrary.RInterpTo` (`SceneComponent.RelativeRotation` (`self.Camera Boom`)) (`|GetArrayItem` (`self.All Dead Camera Views`) (`self.Current Dead Camera View Index`)) (`GameplayStatics.GetWorldDeltaSeconds`) (* (`self.Rotation Speed`) 5.0))))
  (if (`self.Should Allow Player Rotation`)
    (bind (_y _z) (message `/Game/Player/BPI_Player.Get Camera Axis Values` (`self.Owning Player`) :!label _label))
    (`SceneComponent.K2_SetRelativeRotation` (`self.Camera Boom`) (`CustomFunctions.RInterpToConstant` (`KismetMathLibrary.MakeRotator` _relativerotation_roll _relativerotation_pitch _relativerotation_yaw) (`KismetMathLibrary.MakeRotator` 0.0 _y _z) (`GameplayStatics.GetWorldDeltaSeconds`) (`self.Rotation Speed`) true) false false)
    (elif (`KismetArrayLibrary.Array_IsEmpty` (`self.All Dead Camera Views`))
      (goto _label)
      (else
        (`SceneComponent.K2_SetRelativeRotation` (`self.Camera Boom`) (`KismetMathLibrary.MakeRotator` _returnvalue_roll _returnvalue_pitch _returnvalue_yaw) false false)))))

(event `Next Dead Camera View`
  (bind _current_dead_camera_view_index (`self.Current Dead Camera View Index`))
  (if (not (`KismetArrayLibrary.Array_IsEmpty` (`self.All Dead Camera Views`)))
    (set `self.Current Dead Camera View Index` (`KismetMathLibrary.SelectInt` 0 (+ _current_dead_camera_view_index 1) (== (`KismetArrayLibrary.Array_LastIndex` (`self.All Dead Camera Views`)) _current_dead_camera_view_index)))))

(event `Previous Dead Camera View`
  (bind _current_dead_camera_view_index (`self.Current Dead Camera View Index`))
  (if (not (`KismetArrayLibrary.Array_IsEmpty` (`self.All Dead Camera Views`)))
    (set `self.Current Dead Camera View Index` (`KismetMathLibrary.SelectInt` (`KismetArrayLibrary.Array_LastIndex` (`self.All Dead Camera Views`)) (- _current_dead_camera_view_index 1) (== _current_dead_camera_view_index 0)))))

(fn `Find Closest Dead Camera View`
  (locals (`Current Closest` :type "Rotator Structure"))
  (bind (_current_closest_roll _current_closest_pitch _current_closest_yaw) (`KismetMathLibrary.BreakRotator` (`local.Current Closest`)))
  (bind (_relativerotation_roll _relativerotation_pitch _relativerotation_yaw) (`KismetMathLibrary.BreakRotator` (`SceneComponent.RelativeRotation` (`self.Camera Boom`))))
  (bind _returnvalue (`KismetMathLibrary.MakeVector` _relativerotation_roll _relativerotation_pitch _relativerotation_yaw))
  (set `local.Current Closest` (`|GetArrayItem` (`self.All Dead Camera Views`)))
  (for (_array_element _array_index) (`self.All Dead Camera Views`)
    (if (< (`KismetMathLibrary.Vector_Distance` _returnvalue (`KismetMathLibrary.MakeVector` (.roll _array_element) (.pitch _array_element) (.yaw _array_element))) (`KismetMathLibrary.Vector_Distance` (`KismetMathLibrary.MakeVector` _current_closest_roll _current_closest_pitch _current_closest_yaw) _returnvalue))
      (set `local.Current Closest` (`|GetArrayItem` (`self.All Dead Camera Views`) _array_index))))
  (set `self.Current Dead Camera View Index` (`KismetArrayLibrary.Array_Find` (`self.All Dead Camera Views`) (`local.Current Closest`))))

(fn `Find Closest Starting Dead Camera View`
  (locals (`Current Closest Loc` :type "Vector Structure") (`Current Closts Index` :type Integer))
  (bind _returnvalue (`SceneComponent.K2_GetComponentLocation` (`self.Camera`)))
  (bind _returnvalue_2 (`self.K2_GetActorLocation` (`/Game/Player/Health_And_Death/BPC_Player_Health.Owner's Dead Body` (`self.GetComponentByClass` (`self.Owning Player`) "/Game/Player/Health_And_Death/BPC_Player_Health.BPC_Player_Health_C"))))
  (set `local.Current Closest Loc` (0.0 0.0 0.0))
  (for (_array_element _array_index) (`self.All Dead Camera Views`)
    (`SceneComponent.K2_SetRelativeRotation` (`self.Camera Boom`) _array_element false false)
    (if (< (`KismetMathLibrary.Vector_Distance` _returnvalue _returnvalue_2) (`KismetMathLibrary.Vector_Distance` _returnvalue_2 (`local.Current Closest Loc`)))
      (set `local.Current Closest Loc` _returnvalue)
      (set `local.Current Closts Index` _array_index)))
  (set `self.Current Dead Camera View Index` (`local.Current Closts Index`)))

(fn `UserConstructionScript`)