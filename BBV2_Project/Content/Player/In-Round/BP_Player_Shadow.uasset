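; Player drop shadow actor, built around a decal, that shows beneath its owner while airborne and can be activated or deactivated by toggling tick.
; Each tick it box-traces along the owner's orientation-indicator down vector: a wide trace sets its position, offset below the hit, and a narrow one measures height.
; Y/Z scale eases larger with that height and collapses to zero when the owner is grounded or the shadow is deactivated.
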(event `self.ReceiveBeginPlay`
  (bind _static_mesh_component (message `/Game/Player/In-Round/BPI_Player.Get Standard Orientation Indicator` (`self.GetOwner`)))
  (set `self.Owner's Standard Orientation Indicator` _static_mesh_component))

(event `Activate Shadow`
  (`self.SetActorTickEnabled` true))

(event `Deactivate Shadow`
  (`self.SetActorTickEnabled` false)
  (`self.SetActorScale3D` (1.0 0.0 0.0)))

(event `self.ReceiveTick`
  (params (DeltaSeconds :type "Float (single-precision)"))
  (bind (_returnvalue_x _returnvalue_y _returnvalue_z) (`KismetMathLibrary.BreakVector` (`self.GetActorScale3D`)))
  (bind _returnvalue (`GameplayStatics.GetWorldDeltaSeconds`))
  (bind _returnvalue_2 (`self.K2_GetActorLocation` (`self.GetOwner`)))
  (bind _returnvalue_3 (`self.K2_GetActorLocation` (`self.GetOwner`)))
  (`/Engine/EditorBlueprintResources/StandardMacros.IsValid` (`self.GetOwner`)
    (:`Is Valid`
      (bind _on_ground (message `/Game/Player/In-Round/BPI_Player.Get On Ground` (`self.GetOwner`)))
      (if _on_ground
        (`self.SetActorScale3D` (1.0 0.0 0.0))
        (else
          (bind _outhit (`KismetSystemLibrary.BoxTraceSingleForObjects` _returnvalue_3 (+ _returnvalue_3 (* (`SceneComponent.GetUpVector` (`self.Owner's Standard Orientation Indicator`)) -9999.0)) (256.0 256.0 0.0) (struct) (`|MakeArray` "ObjectTypeQuery1" "ObjectTypeQuery2" "ObjectTypeQuery4" :!type "EObjectTypeQuery Enum")))
          (bind _outhit_2 (`KismetSystemLibrary.BoxTraceSingleForObjects` _returnvalue_2 (+ _returnvalue_2 (* (`SceneComponent.GetUpVector` (`self.Owner's Standard Orientation Indicator`)) -9999.0)) (32.0 32.0 0.0) (struct) (`|MakeArray` "ObjectTypeQuery1" "ObjectTypeQuery2" "ObjectTypeQuery4" :!type "EObjectTypeQuery Enum")))
          (`self.K2_SetActorLocation` (- (`.Location` (`GameplayStatics.BreakHitResult` _outhit)) (0.0 0.0 1024.0)))
          (bind _returnvalue_4 (`KismetMathLibrary.MapRangeClamped` (`.Distance` (`GameplayStatics.BreakHitResult` _outhit_2)) 500.0 2500.0 0.0 4.0))
          (`self.SetActorScale3D` (`KismetMathLibrary.MakeVector` 1.0 (`KismetMathLibrary.FInterpTo` _returnvalue_y _returnvalue_4 _returnvalue 5.0) (`KismetMathLibrary.FInterpTo` _returnvalue_z _returnvalue_4 _returnvalue 5.0))))))))

(fn `UserConstructionScript`)