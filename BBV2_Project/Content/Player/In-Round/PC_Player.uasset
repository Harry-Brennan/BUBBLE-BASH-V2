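; In-round player controller that swaps Enhanced Input contexts, toggles scoreboard and pause widgets, and runs the camera flow after death.
; On death, timers hold a ragdoll view, then blend to the level's dead camera, which offers preset views or a rotatable, zoomable mode.
; Spectating retargets the pawn's linked camera to cycle living players.
; A timed lock prevents switching modes mid-blend, and respawning resets the view and state.
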(event `/Game/Player/In-Round/BPI_Player_Controller.Update Input Mapping`
  (params (`New Input Mapping` :type "InputMappingContext Object Reference") (`UI To Focus?` :type "Widget Object Reference"))
  (`/Engine/EditorBlueprintResources/StandardMacros.IsValid` (`self.Current Mapping`)
    (:`Is Valid`
      (`EnhancedInputSubsystemInterface.RemoveMappingContext` (subsystem `EnhancedInputLocalPlayerSubsystem`) (`self.Current Mapping`) (struct))
      (set `self.Current Mapping` null))
    (:`Is Not Valid`
      _))
  (`EnhancedInputSubsystemInterface.AddMappingContext` (subsystem `EnhancedInputLocalPlayerSubsystem`) `New Input Mapping` 0 (struct))
  (set `self.Current Mapping` `New Input Mapping`)
  (`/Engine/EditorBlueprintResources/StandardMacros.IsValid` `UI To Focus?`
    (:`Is Valid`
      (`WidgetBlueprintLibrary.SetInputMode_GameAndUIEx` self `UI To Focus?` "DoNotLock" false)
      (set `self.bShowMouseCursor` true))
    (:`Is Not Valid`
      (`WidgetBlueprintLibrary.SetInputMode_GameOnly` self)
      (set `self.bShowMouseCursor` false))))

(event `Force Close Scoreboard`
  (`Widget.RemoveFromParent` (`self.Scoreboard Widget Ref`) :!label _label))

(event `EnhancedInput|/Game/Player/Input/Actions/Spectating_Dead/IA_Next_Spectating`
  (params (ActionValue :type Boolean) (ElapsedSeconds :type "Float (double-precision)") (TriggeredSeconds :type "Float (double-precision)") (InputAction :type "InputAction Object Reference" :default "/Game/Player/Input/Actions/Spectating_Dead/IA_Next_Spectating.IA_Next_Spectating"))
  (:`Triggered`
    (bind _actor (`self.Find Next Alive Player To Spectate` true))
    (set `self.Currently Spectating Index` (`KismetArrayLibrary.Array_Find` (`self.All Players In Round`) _actor))
    (`/Game/Player/In-Round/BPI_Player_Controller.Update Spectating Target` _actor)))

(event `EnhancedInput|/Game/Player/Input/Actions/Spectating_Dead/IA_Previous_Spectating`
  (params (ActionValue :type Boolean) (ElapsedSeconds :type "Float (double-precision)") (TriggeredSeconds :type "Float (double-precision)") (InputAction :type "InputAction Object Reference" :default "/Game/Player/Input/Actions/Spectating_Dead/IA_Previous_Spectating.IA_Previous_Spectating"))
  (:`Triggered`
    (bind _actor (`self.Find Next Alive Player To Spectate` false))
    (set `self.Currently Spectating Index` (`KismetArrayLibrary.Array_Find` (`self.All Players In Round`) _actor))
    (`/Game/Player/In-Round/BPI_Player_Controller.Update Spectating Target` _actor)))

(event `EnhancedInput|/Game/Player/Input/Actions/Spectating_Dead/IA_Switch_Between_Dead_Spectating`
  (params (ActionValue :type Boolean) (ElapsedSeconds :type "Float (double-precision)") (TriggeredSeconds :type "Float (double-precision)") (InputAction :type "InputAction Object Reference" :default "/Game/Player/Input/Actions/Spectating_Dead/IA_Switch_Between_Dead_Spectating.IA_Switch_Between_Dead_Spectating"))
  (:`Triggered`
    (if (`self.Ragdoll Cam Delay Over?`)
      (if (not (`self.Spectating / Dead Switch Delay`))
        (if (`self.Spectating?`)
          (`/Game/Player/In-Round/BPI_Player_Controller.Switch to Dead` false)
          (else
            (`/Game/Player/In-Round/BPI_Player_Controller.Switch to Spectating`)))
        (set `self.Spectating / Dead Switch Delay` true)
        (`KismetSystemLibrary.K2_SetTimer` null "End Spectating / Dead Switch Delay" (* (`self.Camera Blend Time`) 1.1))
        (set `self.Spectating Zoom Delta` 0.5)))))

(event `/Game/Player/In-Round/BPI_Player_Controller.Switch to Dead`
  (params (`From Actual Death?` :type Boolean))
  (if `From Actual Death?`
    (set `self.Ragdoll Cam Delay Over?` false)
    (`KismetSystemLibrary.K2_SetTimer` null "Prepare Dead Level Cam from Ragdoll" (* (`self.Ragdoll Cam Delay Length`) 0.85))
    (`KismetSystemLibrary.K2_SetTimer` null "End Ragdoll Cam Delay" (`self.Ragdoll Cam Delay Length`))
    (else
      (bind _returnvalue (`GameplayStatics.GetActorOfClass` "/Game/Player/Health_And_Death/BP_Dead_Level_Camera.BP_Dead_Level_Camera_C"))
      (`self.SetViewTargetWithBlend` _returnvalue (`self.Camera Blend Time`) "VTBlend_Cubic")
      (message `/Game/Player/In-Round/BPI_Player.Update Can Change Look Values` (`self.K2_GetPawn`) (`/Game/Player/Health_And_Death/BP_Dead_Level_Camera.Should Allow Player Rotation` _returnvalue))))
  (`/Game/Player/In-Round/BPI_Player_Controller.Update Input Mapping` "/Game/Player/Input/IMC_Dead.IMC_Dead")
  (set `self.Spectating?` false))

(event `/Game/Player/In-Round/BPI_Player_Controller.Switch to Spectating`
  (bind _returnvalue (`self.K2_GetPawn`))
  (bind _outactors (`GameplayStatics.GetAllActorsOfClass` "/Game/Player/In-Round/BP_Player.BP_Player_C"))
  (set `self.All Players In Round` _outactors)
  (message `/Game/Player/In-Round/BPI_Player.Update Can Change Look Values` _returnvalue true)
  (bind _camera (message `/Game/Player/In-Round/BPI_Player.Get Linked Camera` _returnvalue))
  (bind _actor (`self.Find Next Alive Player To Spectate` true))
  (set `self.Currently Spectating Index` (`KismetArrayLibrary.Array_Find` (`self.All Players In Round`) _actor))
  (`self.K2_SetActorLocation` _camera (`self.K2_GetActorLocation` _actor) false false)
  (`self.SetViewTargetWithBlend` _camera (`self.Camera Blend Time`) "VTBlend_Cubic")
  (`/Game/Player/In-Round/BPI_Player_Controller.Update Input Mapping` "/Game/Player/Input/IMC_Spectating.IMC_Spectating")
  (set `self.Spectating?` true)
  (`/Game/Player/In-Round/BPI_Player_Controller.Update Spectating Target` (`|GetArrayItem` (`self.All Players In Round`) (`self.Currently Spectating Index`))))

(event `/Game/Player/In-Round/BPI_Player_Controller.Update Spectating Target`
  (params (`Actor to Spectate` :type "Actor Object Reference"))
  (bind _camera (message `/Game/Player/In-Round/BPI_Player.Get Linked Camera` (`self.K2_GetPawn`)))
  (set `/Game/Player/Camera/BP_Camera.Target Actor` `Actor to Spectate` _camera))

(event `/Game/Player/In-Round/BPI_Player_Controller.Switch from Dead / Spectating to Alive`
  (bind _returnvalue (`self.K2_GetPawn`))
  (message `/Game/Player/In-Round/BPI_Player.Update Can Change Look Values` _returnvalue true)
  (bind _camera (message `/Game/Player/In-Round/BPI_Player.Get Linked Camera` _returnvalue))
  (`/Game/Player/Camera/BP_Camera.Update Alternative Target Arm Length` _camera 0.5 0.01)
  (`self.SetViewTargetWithBlend` _camera (/ (`self.Camera Blend Time`) 4.0) "VTBlend_Cubic")
  (`/Game/Player/In-Round/BPI_Player_Controller.Update Input Mapping` "/Game/Player/Input/IMC_In_Round.IMC_In_Round")
  (set `self.Spectating?` false)
  (set `self.Currently Spectating Index` 0)
  (set `self.Ragdoll Cam Delay Over?` false)
  (set `self.Spectating / Dead Switch Delay` false)
  (bind _returnvalue_2 (`GameplayStatics.GetActorOfClass` "/Game/Player/Health_And_Death/BP_Dead_Level_Camera.BP_Dead_Level_Camera_C"))
  (set `/Game/Player/Health_And_Death/BP_Dead_Level_Camera.Current Dead Camera View Index` 0 _returnvalue_2))

(event `EnhancedInput|/Game/Player/Input/Actions/Spectating_Dead/IA_Next_Dead_Camera_View`
  (params (ActionValue :type Boolean) (ElapsedSeconds :type "Float (double-precision)") (TriggeredSeconds :type "Float (double-precision)") (InputAction :type "InputAction Object Reference" :default "/Game/Player/Input/Actions/Spectating_Dead/IA_Next_Dead_Camera_View.IA_Next_Dead_Camera_View"))
  (:`Triggered`
    (bind _returnvalue (`GameplayStatics.GetActorOfClass` "/Game/Player/Health_And_Death/BP_Dead_Level_Camera.BP_Dead_Level_Camera_C"))
    (`/Game/Player/Health_And_Death/BP_Dead_Level_Camera.Next Dead Camera View` _returnvalue)))

(event `EnhancedInput|/Game/Player/Input/Actions/Spectating_Dead/IA_Previous_Dead_Camera_View`
  (params (ActionValue :type Boolean) (ElapsedSeconds :type "Float (double-precision)") (TriggeredSeconds :type "Float (double-precision)") (InputAction :type "InputAction Object Reference" :default "/Game/Player/Input/Actions/Spectating_Dead/IA_Previous_Dead_Camera_View.IA_Previous_Dead_Camera_View"))
  (:`Triggered`
    (bind _returnvalue (`GameplayStatics.GetActorOfClass` "/Game/Player/Health_And_Death/BP_Dead_Level_Camera.BP_Dead_Level_Camera_C"))
    (`/Game/Player/Health_And_Death/BP_Dead_Level_Camera.Previous Dead Camera View` _returnvalue)))

(event `EnhancedInput|/Game/Player/Input/Actions/Spectating_Dead/IA_Switch_Dead_Camera_Mode`
  (params (ActionValue :type Boolean) (ElapsedSeconds :type "Float (double-precision)") (TriggeredSeconds :type "Float (double-precision)") (InputAction :type "InputAction Object Reference" :default "/Game/Player/Input/Actions/Spectating_Dead/IA_Switch_Dead_Camera_Mode.IA_Switch_Dead_Camera_Mode"))
  (:`Triggered`
    (bind _returnvalue (`GameplayStatics.GetActorOfClass` "/Game/Player/Health_And_Death/BP_Dead_Level_Camera.BP_Dead_Level_Camera_C"))
    (bind _should_allow_player_rotation (`/Game/Player/Health_And_Death/BP_Dead_Level_Camera.Should Allow Player Rotation` _returnvalue))
    (if _should_allow_player_rotation
      (message `/Game/Player/In-Round/BPI_Player.Update Can Change Look Values` (`self.K2_GetPawn`) false)
      (`/Game/Player/Health_And_Death/BP_Dead_Level_Camera.Find Closest Dead Camera View` _returnvalue)
      (set `/Game/Player/Health_And_Death/BP_Dead_Level_Camera.Zoom Percentage` 0.5 _returnvalue)
      (else
        (bind (_relativerotation_roll _relativerotation_pitch _relativerotation_yaw) (`KismetMathLibrary.BreakRotator` (`SceneComponent.RelativeRotation` (`/Game/Player/Health_And_Death/BP_Dead_Level_Camera.Camera Boom` _returnvalue))))
        (message `/Game/Player/In-Round/BPI_Player.Update Camera Axis Values` (`self.K2_GetPawn`) _relativerotation_pitch _relativerotation_yaw 0.25)
        (`/Game/Player/Health_And_Death/BP_Dead_Level_Camera.Update Zoom Percentage` _returnvalue 0.5)))
    (set `/Game/Player/Health_And_Death/BP_Dead_Level_Camera.Should Allow Player Rotation` (not _should_allow_player_rotation) _returnvalue)
    (set `self.Spectating Zoom Delta` 0.5)))

(event `EnhancedInput|/Game/Player/Input/Actions/Spectating_Dead/IA_Scroll_Camera_Zoom`
  (params (ActionValue :type "Float (double-precision)") (ElapsedSeconds :type "Float (double-precision)") (TriggeredSeconds :type "Float (double-precision)") (InputAction :type "InputAction Object Reference" :default "/Game/Player/Input/Actions/Spectating_Dead/IA_Scroll_Camera_Zoom.IA_Scroll_Camera_Zoom"))
  (bind _returnvalue (+ (* ActionValue -0.1) (`self.Spectating Zoom Delta`) (`GameplayStatics.GetWorldDeltaSeconds`)))
  (:`Triggered`
    (if (`self.Spectating?`)
      (set `self.Spectating Zoom Delta` (`KismetMathLibrary.FClamp` _returnvalue))
      (bind _camera (message `/Game/Player/In-Round/BPI_Player.Get Linked Camera` (`self.K2_GetPawn`)))
      (`/Game/Player/Camera/BP_Camera.Update Alternative Target Arm Length` _camera (`self.Spectating Zoom Delta`) (`self.Spectating Zoom Time Until Back To Normal`))
      (`KismetSystemLibrary.RetriggerableDelay` (`self.Spectating Zoom Time Until Back To Normal`))
      (set `self.Spectating Zoom Delta` 0.5)
      (else
        (bind _returnvalue_2 (`GameplayStatics.GetActorOfClass` "/Game/Player/Health_And_Death/BP_Dead_Level_Camera.BP_Dead_Level_Camera_C"))
        (if (`/Game/Player/Health_And_Death/BP_Dead_Level_Camera.Should Allow Player Rotation` _returnvalue_2)
          (bind _output_get (set `self.Spectating Zoom Delta` (`KismetMathLibrary.FClamp` _returnvalue)))
          (`/Game/Player/Health_And_Death/BP_Dead_Level_Camera.Update Zoom Percentage` _returnvalue_2 _output_get))))))

(event `EnhancedInput|/Game/Player/Input/Actions/In_Round/IA_Scoreboard_Toggle`
  (params (ActionValue :type Boolean) (ElapsedSeconds :type "Float (double-precision)") (TriggeredSeconds :type "Float (double-precision)") (InputAction :type "InputAction Object Reference" :default "/Game/Player/Input/Actions/In_Round/IA_Scoreboard_Toggle.IA_Scoreboard_Toggle"))
  (bind _scoreboard_widget_ref (`self.Scoreboard Widget Ref`))
  (:`Triggered`
    (`/Engine/EditorBlueprintResources/StandardMacros.IsValid` _scoreboard_widget_ref
      (:`Is Valid`
        (if (`Widget.IsInViewport` _scoreboard_widget_ref)
          (goto _label)
          (else
            (`UserWidget.AddToViewport` (`self.Scoreboard Widget Ref`) 0))))
      (:`Is Not Valid`
        (bind _returnvalue (`|CreateWidget` "/Game/UI/In_Round/Scoreboard/WBP_Scoreboard_Main.WBP_Scoreboard_Main_C"))
        (bind _output_get (set `self.Scoreboard Widget Ref` _returnvalue))
        (`UserWidget.AddToViewport` _returnvalue 0)
        (`UserWidget.AddToViewport` _output_get 0)))))

(event `Force Close Pause Menu`
  (`Widget.RemoveFromParent` (`self.Pause Widget Ref`) :!label _label_2)
  (`WidgetBlueprintLibrary.SetInputMode_GameOnly` self)
  (set `self.bShowMouseCursor` false))

(event `EnhancedInput|/Game/Player/Input/Actions/In_Round/IA_Pause`
  (params (ActionValue :type Boolean) (ElapsedSeconds :type "Float (double-precision)") (TriggeredSeconds :type "Float (double-precision)") (InputAction :type "InputAction Object Reference" :default "/Game/Player/Input/Actions/In_Round/IA_Pause.IA_Pause"))
  (bind _pause_widget_ref (`self.Pause Widget Ref`))
  (:`Triggered`
    (`/Engine/EditorBlueprintResources/StandardMacros.IsValid` _pause_widget_ref
      (:`Is Valid`
        (if (`Widget.IsInViewport` _pause_widget_ref)
          (goto _label_2)
          (else
            (`UserWidget.AddToViewport` (`self.Pause Widget Ref`) 0)
            (`WidgetBlueprintLibrary.SetInputMode_UIOnlyEx` self (`self.Pause Widget Ref`))
            (set `self.bShowMouseCursor` true))))
      (:`Is Not Valid`
        (bind _returnvalue (`|CreateWidget` "/Game/UI/In_Round/Pause/WBP_Pause_Menu.WBP_Pause_Menu_C"))
        (bind _output_get (set `self.Pause Widget Ref` _returnvalue))
        (`UserWidget.AddToViewport` _output_get 0)
        (`WidgetBlueprintLibrary.SetInputMode_UIOnlyEx` self (`self.Pause Widget Ref`))
        (set `self.bShowMouseCursor` true)))))

(fn `End Ragdoll Cam Delay`
  (set `self.Ragdoll Cam Delay Over?` true)
  (message `/Game/Player/In-Round/BPI_Player.Update Can Change Look Values` (`self.K2_GetPawn`) false)
  (bind _returnvalue (`GameplayStatics.GetActorOfClass` "/Game/Player/Health_And_Death/BP_Dead_Level_Camera.BP_Dead_Level_Camera_C"))
  (`self.SetViewTargetWithBlend` _returnvalue (`self.Camera Blend Time`) "VTBlend_Cubic")
  (set `self.Spectating / Dead Switch Delay` true)
  (`KismetSystemLibrary.K2_SetTimer` null "End Spectating / Dead Switch Delay" (* (`self.Camera Blend Time`) 1.5)))

(fn `End Spectating / Dead Switch Delay`
  (set `self.Spectating / Dead Switch Delay` false))

(fn `Find Next Alive Player To Spectate`
  (params (`Next?` :type Boolean))
  (returns (Actor :type "Actor Object Reference"))
  (locals (`Current Next` :type "Actor Object Reference") (`Reversed Players In Round` :type "Array of Actor Object Reference") (`Reversed Current Spectating Index` :type Integer))
  (if `Next?`
    (for (_array_element _array_index) (`self.All Players In Round`)
      (if (and (`/Game/Player/Health_And_Death/BPC_Player_Health.Player Alive?` (`self.GetComponentByClass` _array_element "/Game/Player/Health_And_Death/BPC_Player_Health.BPC_Player_Health_C")) (> (`self.Currently Spectating Index`) _array_index))
        (set `local.Current Next` _array_element)))
    (else
      (bind _output_get (set `local.Reversed Players In Round` (`self.All Players In Round`)))
      (`KismetArrayLibrary.Array_Reverse` _output_get)
      (set `local.Reversed Current Spectating Index` (`KismetArrayLibrary.Array_Find` (`local.Reversed Players In Round`) (`|GetArrayItem` (`self.All Players In Round`) (`self.Currently Spectating Index`))))
      (for (_array_element_2 _array_index_2) (`local.Reversed Players In Round`)
        (if (and (`/Game/Player/Health_And_Death/BPC_Player_Health.Player Alive?` (`self.GetComponentByClass` _array_element_2 "/Game/Player/Health_And_Death/BPC_Player_Health.BPC_Player_Health_C")) (< _array_index_2 (`local.Reversed Current Spectating Index`)))
          (set `local.Current Next` _array_element_2)))))
  (`/Engine/EditorBlueprintResources/StandardMacros.IsValid` (`local.Current Next`)
    (:`Is Valid`
      (return (`local.Current Next`)))
    (:`Is Not Valid`
      (if (`local.Next?`)
        (for _array_element_3 (`self.All Players In Round`)
          (if (`/Game/Player/Health_And_Death/BPC_Player_Health.Player Alive?` (`self.GetComponentByClass` _array_element_3 "/Game/Player/Health_And_Death/BPC_Player_Health.BPC_Player_Health_C"))
            (set `local.Current Next` _array_element_3)))
        (else
          (for _array_element_4 (`local.Reversed Players In Round`)
            (if (`/Game/Player/Health_And_Death/BPC_Player_Health.Player Alive?` (`self.GetComponentByClass` _array_element_4 "/Game/Player/Health_And_Death/BPC_Player_Health.BPC_Player_Health_C"))
              (set `local.Current Next` _array_element_4)))))
      (`/Engine/EditorBlueprintResources/StandardMacros.IsValid` (`local.Current Next`)
        (:`Is Valid`
          (return (`local.Current Next`)))
        (:`Is Not Valid`
          (return (`|GetArrayItem` (`self.All Players In Round`) (`self.Currently Spectating Index`))))))))

(fn `Prepare Dead Level Cam from Ragdoll`
  (bind _returnvalue (`GameplayStatics.GetActorOfClass` "/Game/Player/Health_And_Death/BP_Dead_Level_Camera.BP_Dead_Level_Camera_C"))
  (`/Game/Player/Health_And_Death/BP_Dead_Level_Camera.Find Closest Starting Dead Camera View` _returnvalue)
  (`/Game/Player/Health_And_Death/BP_Dead_Level_Camera.Activate Dead Level Cam` _returnvalue))

(fn `UserConstructionScript`)