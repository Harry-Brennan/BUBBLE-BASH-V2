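; BP_Player_Main_Menu is the player Blueprint for the main menu, providing camera look and interaction with widgets through a WidgetInteraction component.
; BeginPlay sets game-only or game-and-UI input from InputMode, and IA_Look rotates the spring arm with clamped pitch while CanLook is set.
; IA_UI_Interact simulates left-mouse presses on the WidgetInteraction, which events can enable or disable.
; A debug C key opens the customisation widget in UI-only mode.
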(event Custom|Disable%20Widget%20Interaction
  (Components|Activation|Deactivate (Variables|Default|GetWidgetInteraction)))

(event Custom|Enable%20Widget%20Interaction
  (Components|Activation|Activate (Variables|Default|GetWidgetInteraction) true))

(event Input|EnhancedActionEvents|EnhancedInputActionIA_Look
  (params (ActionValue :type Vector%202D%20Structure) (ElapsedSeconds :type Float%20%28double-precision%29) (TriggeredSeconds :type Float%20%28double-precision%29) (InputAction :type Input%20Action%20Object%20Reference :default "/Game/Player/Input/Actions/IA_Look.IA_Look"))
  (bind _springarm (Variables|Default|GetSpringArm))
  (bind _relativerotation (Variables|/Script/Engine.SceneComponent|GetRelativeRotation _springarm))
  ;[0 0 0] CAMERA ROTATION
  (if (Variables|Default|GetCan%20Look?)
    (Transformation|SetWorldRotation (Variables|Default|GetSpringArm) (Math|Rotator|MakeRotator 0.0 (Math|Float|Clamp(Float) (+ (.pitch _relativerotation) (* (.y ActionValue) 5.0)) -6e+01 6e+01) (+ (.yaw _relativerotation) (* (.x ActionValue) 5.0))) false false)))

(event Input|EnhancedActionEvents|EnhancedInputActionIA_UI_Interact
  (params (ActionValue :type Boolean) (ElapsedSeconds :type Float%20%28double-precision%29) (TriggeredSeconds :type Float%20%28double-precision%29) (InputAction :type Input%20Action%20Object%20Reference :default "/Game/Player/Input/Actions/Main_Menu/IA_UI_Interact.IA_UI_Interact"))
  (bind _widgetinteraction (Variables|Default|GetWidgetInteraction))
  (:Triggered
    (Class|WidgetInteractionComponent|PressPointerKey _widgetinteraction "LeftMouseButton"))
  (:Canceled
    (Class|WidgetInteractionComponent|ReleasePointerKey _widgetinteraction "LeftMouseButton" :!label _label))
  (:Completed
    (goto _label)))

(event EventBeginPlay
  (bind _returnvalue (Game|GetPlayerController 0))
  (if (== (Variables|Default|GetInput%20Mode) 0)
    (Input|SetInputModeGameOnly _returnvalue false)
    (else
      (Input|SetInputModeGameandUI _returnvalue 0 "DoNotLock" true false)
      (Variables|/Script/Engine.PlayerController|SetbShowMouseCursor _returnvalue true))))

(event Input|KeyboardEvents|DebugKeyC
  (params (Key :type Key%20Structure :default "None") (ActionValue :type Input%20Action%20Value%20Structure))
  (bind _returnvalue (Game|GetPlayerController 0))
  (:Pressed
    (bind _returnvalue_2 (UserInterface|CreateWidget "/Game/UI/Main_Menu/Customisation/WBP_Customisation_Main.WBP_Customisation_Main_C"))
    (UserInterface|Viewport|AddtoViewport _returnvalue_2 0)
    (Input|SetInputModeUIOnly _returnvalue _returnvalue_2 "DoNotLock" false)
    (Variables|/Script/Engine.PlayerController|SetbShowMouseCursor _returnvalue true)))

(fn ConstructionScript)