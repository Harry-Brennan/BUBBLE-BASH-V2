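; Player health component that handles the owning pawn's death and revival, caching its controller at BeginPlay.
; Death switches to a dead input mapping, hides the pawn, disables collision and gravity, and spawns a BP_Dead_Player body launched with the pawn's velocity.
; The linked camera is retargeted to that body through interface messages.
; ResetHealth restores input, visibility, collision, gravity and camera target without removing the body.
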(event `self.ReceiveBeginPlay`
  (bind _aspawn (cast `Pawn` (`self.GetOwner`)))
  (set `self.Owner's Controller` (`Pawn.GetController` _aspawn)))

(fn `Death`
  (bind _returnvalue (`self.GetOwner`))
  (set `self.Player Alive?` false)
  (message `/Game/Player/BPI_Player_Controller.Update Input Mapping` (`self.Owner's Controller`) "/Game/Player/Input/IMC_Dead.IMC_Dead" null)
  (bind _visible_mesh_ref (message `/Game/Player/BPI_Player.Get Visible Mesh` (`self.GetOwner`)))
  (bind (_returnvalue_location _returnvalue_rotation) (`KismetMathLibrary.BreakTransform` (`SceneComponent.K2_GetComponentToWorld` _visible_mesh_ref)))
  (bind _returnvalue_2 (`|SpawnActorFromClass` "/Game/Player/BP_Dead_Player.BP_Dead_Player_C" (`KismetMathLibrary.MakeTransform` _returnvalue_location _returnvalue_rotation) "Undefined" "MultiplyWithRoot" null "NewEnumerator0" null))
  (`Actor.SetActorEnableCollision` _returnvalue false)
  (`Actor.SetActorHiddenInGame` _returnvalue true)
  (`PrimitiveComponent.AddImpulse` (`/Game/Player/BP_Dead_Player.Dead Mesh` _returnvalue_2) (* (`Actor.GetVelocity` (`self.GetOwner`)) 3.0) "None" true)
  (bind _ascapsule_collision (cast `CapsuleComponent` (`Actor.RootComponent` (`self.GetOwner`))))
  (`PrimitiveComponent.SetEnableGravity` _ascapsule_collision false)
  (`PrimitiveComponent.SetAllPhysicsLinearVelocity` _ascapsule_collision (0.0 0.0 0.0) false)
  (bind _camera (message `/Game/Player/BPI_Player.Get Linked Camera` (`self.GetOwner`)))
  (`/Game/Player/BP_Camera.Update Target Actor` _camera _returnvalue_2))

(fn `Reset Health`
  (bind _returnvalue (`self.GetOwner`))
  (bind _returnvalue_2 (`self.GetOwner`))
  (set `self.Player Alive?` true)
  (message `/Game/Player/BPI_Player_Controller.Update Input Mapping` (`self.Owner's Controller`) "/Game/Player/Input/IMC_In_Round.IMC_In_Round" null)
  (`Actor.SetActorEnableCollision` _returnvalue_2 true)
  (`Actor.SetActorHiddenInGame` _returnvalue_2 false)
  (bind _ascapsule_collision (cast `CapsuleComponent` (`Actor.RootComponent` (`self.GetOwner`))))
  (`PrimitiveComponent.SetEnableGravity` _ascapsule_collision true)
  (bind _camera (message `/Game/Player/BPI_Player.Get Linked Camera` _returnvalue))
  (`/Game/Player/BP_Camera.Update Target Actor` _camera _returnvalue))