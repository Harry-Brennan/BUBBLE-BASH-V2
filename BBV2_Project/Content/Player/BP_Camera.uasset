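; Player follow camera actor that trails a target actor, initially its owner, which can be swapped through UpdateTargetActor.
; Each tick, the spring arm rotates at constant speed toward pitch and yaw values polled from the owning player.
; Arm length eases with target speed, with vertical velocity scaled by a divisor.
; Location interpolates separately: horizontal follow speed scales with planar distance to the target, vertical with the target's vertical velocity.
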(event `Update Target Actor`
  (params (`New Target` :type "Actor Object Reference"))
  (set `self.Target Actor` `New Target`))

(event `self.ReceiveBeginPlay`
  (bind _output_get (set `self.Target Actor` (`self.GetOwner`)))
  (set `self.Owning Player` _output_get))

(event `self.ReceiveTick`
  (params (DeltaSeconds :type "Float (single-precision)"))
  (bind (_returnvalue_x _returnvalue_y) (`KismetMathLibrary.BreakVector` (`self.K2_GetActorLocation`)))
  (bind (_returnvalue_x_2 _returnvalue_y_2 _returnvalue_z) (`KismetMathLibrary.BreakVector` (`self.GetVelocity` (`self.Target Actor`))))
  (bind (_returnvalue_x_3 _returnvalue_y_3) (`KismetMathLibrary.BreakVector` (`self.K2_GetActorLocation` (`self.Target Actor`))))
  (bind (_returnvalue_x_4 _returnvalue_y_4 _returnvalue_z_2) (`KismetMathLibrary.BreakVector` (`self.GetVelocity` (`self.Target Actor`))))
  (bind (_returnvalue_x_5 _returnvalue_y_5) (`KismetMathLibrary.BreakVector` (`KismetMathLibrary.VInterpTo` (`self.K2_GetActorLocation`) (`self.K2_GetActorLocation` (`self.Target Actor`)) (`GameplayStatics.GetWorldDeltaSeconds`) (`KismetMathLibrary.MapRangeClamped` (`KismetMathLibrary.Vector_Distance` (`KismetMathLibrary.MakeVector` _returnvalue_x _returnvalue_y) (`KismetMathLibrary.MakeVector` _returnvalue_x_3 _returnvalue_y_3)) 0.0 (`self.Max XY Velocity Range`) (`self.Min Camera XY Move Speed`) (`self.Max Camera XY Move Speed`)))))
  (bind (_returnvalue_x_6 _returnvalue_y_6 _returnvalue_z_3) (`KismetMathLibrary.BreakVector` (`KismetMathLibrary.VInterpTo` (`self.K2_GetActorLocation`) (`self.K2_GetActorLocation` (`self.Target Actor`)) (`GameplayStatics.GetWorldDeltaSeconds`) (`KismetMathLibrary.MapRangeClamped` (`KismetMathLibrary.VSize` (`KismetMathLibrary.MakeVector` _returnvalue_z_2)) 0.0 (`self.Max Z Velocity Range`) (`self.Min Camera Z Move Speed`) (`self.Max Camera Z Move Speed`)))))
  (bind (_y _z) (message `/Game/Player/BPI_Player.Get Camera Axis Values` (`self.Owning Player`)))
  (`SceneComponent.K2_SetRelativeRotation` (`self.Camera Boom`) (`CustomFunctions.RInterpToConstant` (`SceneComponent.RelativeRotation` (`self.Camera Boom`)) (`KismetMathLibrary.MakeRotator` 0.0 _y _z) (`GameplayStatics.GetWorldDeltaSeconds`) (`self.Rotation Speed`) true) false false)
  (set `SpringArmComponent.TargetArmLength` (`KismetMathLibrary.FInterpTo` (`SpringArmComponent.TargetArmLength` (`self.Camera Boom`)) (`KismetMathLibrary.MapRangeClamped` (`KismetMathLibrary.VSize` (`KismetMathLibrary.MakeVector` _returnvalue_x_2 _returnvalue_y_2 (/ _returnvalue_z (`self.Arm Length Z Velocity Division Factor`)))) 0.0 (`self.Max Velocity Arm Equivalent`) (`self.Min Arm Length`) (`self.Max Arm Length`)) (`GameplayStatics.GetWorldDeltaSeconds`) (`self.Arm Length Interp Speed`)) (`self.Camera Boom`))
  (`self.K2_SetActorLocation` (`KismetMathLibrary.MakeVector` _returnvalue_x_5 _returnvalue_y_5 _returnvalue_z_3)))

(fn `UserConstructionScript`)