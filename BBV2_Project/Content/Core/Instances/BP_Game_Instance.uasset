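; Game instance that carries game state and per-player state data across map changes and chooses the next map.
; Before travel, it snapshots persistent info messages from the game state and every player state, storing player entries by index.
; It then picks a random DT_Map_Info row and one of its possible modes, stores the mode for later query, and opens that level.
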(event `/Game/Core/Instances/BPI_Game_Instance.Set Game Instance Persistent Info`
  (params (`Game State Persistent Info` :type "/Game/Core/Game_States/Struct_Persistent_Game_State_Info Structure") (`Player State Persistent Info` :type "Array of /Game/Core/Player_States/Struct_Persistent_Player_State_Info Structure (by ref)"))
  (set `self.Game State Persistent Info` `Game State Persistent Info`)
  (set `self.Player State Persistent Info` `Player State Persistent Info`))

(event `self.ReceiveInit`
  (`KismetSystemLibrary.PrintString` "GAME INSTANCE INITIALISED"))

(event `/Game/Core/Instances/BPI_Game_Instance.Set Persistent Data`
  (bind _persistent_game_state_info (message `/Game/Core/Game_States/BPI_Standard_GS.Get Persistent Game State Info` (`GameplayStatics.GetGameState`)))
  (set `self.Game State Persistent Info` _persistent_game_state_info)
  (for _index (range (`GameplayStatics.GetNumPlayerStates`))
    (bind _persistent_player_state_info (message `/Game/Core/Player_States/BPI_Standard_PS.Get Persistent Player State Info` (`GameplayStatics.GetPlayerState` _index)))
    (if (`KismetArrayLibrary.Array_IsValidIndex` (`self.Player State Persistent Info`) _index)
      (`KismetArrayLibrary.Array_Set` (`self.Player State Persistent Info`) _index _persistent_player_state_info)
      (else
        (`KismetArrayLibrary.Array_Add` (`self.Player State Persistent Info`) _persistent_player_state_info)))))

(event `/Game/Core/Instances/BPI_Game_Instance.Determine and Open Next Map`
  (`self.Set Persistent Data`)
  (bind _outrownames (`DataTableFunctionLibrary.GetDataTableRowNames` "/Game/Core/Maps/DT_Map_Info.DT_Map_Info"))
  (bind _returnvalue (`|GetDataTableRow` "/Game/Core/Maps/DT_Map_Info.DT_Map_Info" (`KismetArrayLibrary.Array_Random` _outrownames))
    (:`then`
      (bind (_level _possiblemodes) (break `/Game/Core/Maps/Struct_Map_Info` _returnvalue))
      (set `self.Next Map Mode` (`KismetArrayLibrary.Array_Random` _possiblemodes))
      (`GameplayStatics.OpenLevelBySoftObjectPtr` (`.WorldAsset` (break `SoftWorldReference` _level))))))

(fn `Get Current Level Mode`
  (returns (`Level Mode` :type "/Game/Core/Enum_Level_Modes Enum"))
  (return (`self.Next Map Mode`)))

(fn `Get Game Instance Persistent Info`
  (returns (`Game State Persistent Info` :type "/Game/Core/Game_States/Struct_Persistent_Game_State_Info Structure") (`Player State Persistent Info` :type "Array of /Game/Core/Player_States/Struct_Persistent_Player_State_Info Structure"))
  (return (`self.Game State Persistent Info`) (`self.Player State Persistent Info`)))