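; GM_In_Round is the in-round game mode that restores persistent game and player info when play begins.
; On BeginPlay it reads the persistent info message from the game instance and passes the game-state part to the game state.
; If the per-player array is not empty, it hands each player state the entry at the same index, relying on matching order without a length check.
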(event `self.ReceiveBeginPlay`
  (`KismetSystemLibrary.PrintString` "GAME MODE BEGINPLAY")
  (bind (_game_state_persistent_info _player_state_persistent_info) (message `/Game/Core/Instances/BPI_Game_Instance.Get Game Instance Persistent Info` (`GameplayStatics.GetGameInstance`)))
  (message `/Game/Core/Game_States/BPI_Standard_GS.Set Persistent Game State Info` (`GameplayStatics.GetGameState`) _game_state_persistent_info)
  (if (not (`KismetArrayLibrary.Array_IsEmpty` _player_state_persistent_info))
    (for _index (range (`GameplayStatics.GetNumPlayerStates`))
      (message `/Game/Core/Player_States/BPI_Standard_PS.Set Persistent Player State Info` (`GameplayStatics.GetPlayerState` _index) (`|GetArrayItem` _player_state_persistent_info _index)))))

(fn `UserConstructionScript`)