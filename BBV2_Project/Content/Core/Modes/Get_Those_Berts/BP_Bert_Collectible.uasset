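; BP_Bert_Collectible is a pickup actor for the Get Those Berts mode.
; Enabling it sets Active, moves it to a given transform, and makes it visible and collidable.
; Any overlap on BertCollectionCollision reports the overlapping actor to the GameState via PlayerCollectedBertMessage, then calls DisableBertCollectible.
; Disabling only clears Active, leaving the actor visible and collidable, and the overlap handler never checks that flag.
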(event `Enable Bert Collectible`
  (params (`New Transform` :type "Transform Structure"))
  (set `self.Active?` true)
  (`self.K2_SetActorTransform` `New Transform`)
  (`self.SetActorEnableCollision` true)
  (`self.SetActorHiddenInGame` false))

(event `Disable Bert Collectible`
  (set `self.Active?` false)
  (`self.SetActorEnableCollision` true)
  (`self.SetActorHiddenInGame` false))

(event `self.Bert Collection Collision.OnComponentBeginOverlap`
  (params (OverlappedComponent :type "PrimitiveComponent Object Reference") (OtherActor :type "Actor Object Reference") (OtherComp :type "PrimitiveComponent Object Reference") (OtherBodyIndex :type Integer) (bFromSweep :type Boolean) (SweepResult :type "HitResult Structure (by ref)"))
  (message `/Game/Core/Game_States/BPI_Standard_GS.Player Collected Bert` (`GameplayStatics.GetGameState`) OtherActor)
  (`self.Disable Bert Collectible`))

(fn `UserConstructionScript`)